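; Game manager Blueprint that tracks a Running, Win, Lose or Abandon state and switches end-screen UI to match.
; Init creates the three end-screen widgets and enters Running.
; SetState hides the UI, then on a change shows the matching widget and cursor, or hides the cursor for Running.
; ResetGame teleports the player to the first PlayerStart found and reruns Init, creating the widgets again.
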(fn `Create UI`
  (bind _returnvalue (`|CreateWidget` "/Game/_MyContent/UI/Widget_Abandon.Widget_Abandon_C"))
  (bind _output_get (set `self.WidgetAbandon` _returnvalue))
  (`UserWidget.AddToViewport` _output_get 0)
  (bind _returnvalue_2 (`|CreateWidget` "/Game/_MyContent/UI/Widget_Lose.Widget_Lose_C"))
  (bind _output_get_2 (set `self.WidgetLose` _returnvalue_2))
  (`UserWidget.AddToViewport` _output_get_2 0)
  (bind _returnvalue_3 (`|CreateWidget` "/Game/_MyContent/UI/Widget_Win.Widget_Win_C"))
  (bind _output_get_3 (set `self.WidgetWin` _returnvalue_3))
  (`UserWidget.AddToViewport` _output_get_3 0))

(fn `Get State`
  (returns (State :type "/Game/_MyContent/Blueprints/E_MyGameState Enum"))
  (return (`self.CurrentGameState`)))

(fn `Init`
  (`self.Create UI`)
  (`self.Set State` "NewEnumerator0"))

(fn `Reset Game`
  (bind _outactors (`GameplayStatics.GetAllActorsOfClass` "/Script/Engine.PlayerStart"))
  (`self.K2_SetActorLocation` (`self.MyPlayer`) (`self.K2_GetActorLocation` (`|GetArrayItem` _outactors)) false false)
  (bind _my_game_manager (`/Game/_MyContent/Blueprints/BP_MyFunctionLibrary.Get My Game Manager`))
  (`self.Init` _my_game_manager))

(fn `Set State`
  (params (`New State` :type "/Game/_MyContent/Blueprints/E_MyGameState Enum" :default "NewEnumerator0"))
  (`/Game/_MyContent/Blueprints/BP_MyFunctionLibrary.Hide UI`)
  (if (`|EnumInequality` `New State` (`self.CurrentGameState`))
    (bind _output_get (set `self.CurrentGameState` `New State`))
    (switch `/Game/_MyContent/Blueprints/E_MyGameState` _output_get
      (:`NewEnumerator0`
        (`/Game/_MyContent/Blueprints/BP_MyFunctionLibrary.Show Mouse` false))
      (:`NewEnumerator1`
        (`Widget.SetVisibility` (`self.WidgetWin`) "Visible")
        (`/Game/_MyContent/Blueprints/BP_MyFunctionLibrary.Show Mouse` true :!label _label))
      (:`NewEnumerator2`
        (`Widget.SetVisibility` (`self.WidgetLose`) "Visible")
        (goto _label))
      (:`NewEnumerator3`
        (`Widget.SetVisibility` (`self.WidgetAbandon`) "Visible")
        (goto _label)))))

(fn `UserConstructionScript`)