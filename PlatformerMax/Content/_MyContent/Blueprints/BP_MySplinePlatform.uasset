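; A moving platform actor that travels along a spline, starting automatically on BeginPlay.
; A timeline, with its play rate set from a Rate variable, outputs a normalized distance that is scaled by spline length to position the platform mesh in world space each update, without sweeping.
; The construction script applies the configurable static mesh and material to the platform.
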(event `self.ReceiveBeginPlay`
  (`self.Platform start`))

(event `Platform start`
  (bind _spline (`self.Spline`))
  (`TimelineComponent.SetPlayRate` (`self.Motion timeline`) (`self.Rate`))
  (bind (_direction _spline_distance) (`Timeline|Motion timeline`)
    (:`Update`
      (`SceneComponent.K2_SetWorldLocation` (`self.Platform mesh`) (`SplineComponent.GetLocationAtDistanceAlongSpline` _spline (* _spline_distance (`SplineComponent.GetSplineLength` _spline)) "World") false false))))

(fn `UserConstructionScript`
  (bind _platform_mesh (`self.Platform mesh`))
  (`StaticMeshComponent.SetStaticMesh` _platform_mesh (`self.Static mesh`))
  (`PrimitiveComponent.SetMaterial` _platform_mesh 0 (`self.Material`)))